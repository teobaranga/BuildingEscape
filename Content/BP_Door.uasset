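; BP_Door is a door actor that swings open and closed around its yaw axis from its starting rotation.
; OnOpen plays a timeline that adds an angle to the rotation cached at BeginPlay, with an event track firing a lock sound at the door's location.
; OnClose waits briefly, then reverses the same timeline at a faster play rate.
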(event `self.ReceiveBeginPlay`
  (set `self.InitialRotation` (`self.K2_GetActorRotation`)))

(event `self.Door.OnOpen`
  (`TimelineComponent.SetPlayRate` (`self.Timeline`) 1.0)
  (bind (_direction _open_angle) (`Timeline|Timeline` :!label _label)
    (:`Update`
      (`self.K2_SetActorRotation` (`KismetMathLibrary.ComposeRotators` (`self.InitialRotation`) (`KismetMathLibrary.MakeRotator` 0.0 0.0 _open_angle))))
    (:`Sound timing`
      (`GameplayStatics.PlaySoundAtLocation` "/Game/Audio/door-lock.door-lock" (`self.K2_GetActorLocation`)))))

(event `self.Door.OnClose`
  (`TimelineComponent.SetPlayRate` (`self.Timeline`) 4.0)
  (`KismetSystemLibrary.Delay` 0.5)
  (goto _label :!via `Reverse`))

(fn `UserConstructionScript`)